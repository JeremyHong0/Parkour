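; GA_Test is a gameplay ability that dashes the avatar forward, then performs a melee attack.
; After committing, constant-force root motion runs alongside a short-mantle montage, whose finish switches to a named section of the melee combo montage.
; A one-shot Event.Damage listener applies GE_DealDamage to the event's target, passing damage as a SetByCaller magnitude.
; The ability ends when the attack montage finishes or is interrupted, or if commit fails.
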(event `self.K2_ActivateAbility`
  (bind _returnvalue (`self.K2_CommitAbility`))
  (if _returnvalue
    (`AbilityTask_ApplyRootMotionConstantForce.ApplyRootMotionConstantForce` "None" (`Actor.GetActorForwardVector` (`self.GetAvatarActorFromActorInfo`)) 1200.0 0.5 false null "MaintainLastRootMotionVelocity"
      (:`then`
        (`AbilityTask_PlayMontageAndWait.CreatePlayMontageAndWaitProxy` "None" "/Game/Character/Mannequin/Animations/Mantle/AM_ProxyShortMantle.AM_ProxyShortMantle"))
      (:`OnFinish`
        (`self.MontageStop` -1.0)
        (`AbilityTask_PlayMontageAndWait.CreatePlayMontageAndWaitProxy` "None" "/Game/Character/Mannequin/Animations/Attack/AM_Melee_Combo.AM_Melee_Combo" 1.0 (`self.Attack Montage Section Name`) false
          (:`then`
            (bind (_asynctaskproxy _payload) (`AbilityTask_WaitGameplayEvent.WaitGameplayEvent` (struct :`TagName` "Event.Damage") null true)
              (:`EventReceived`
                (bind _result (`/Engine/EditorBlueprintResources/StandardMacros.NegateFloat` (`self.Damage`))
                  (:`  `
                    (bind _returnvalue_2 (`AbilitySystemBlueprintLibrary.AssignTagSetByCallerMagnitude` (`self.MakeOutgoingGameplayEffectSpec` "/Game/GE_DealDamage.GE_DealDamage_C") (struct :`TagName` "Event.Damage") _result))
                    (`AbilitySystemComponent.BP_ApplyGameplayEffectSpecToTarget` (`AbilitySystemBlueprintLibrary.GetAbilitySystemComponent` (`self.GetAvatarActorFromActorInfo`)) _returnvalue_2 (`AbilitySystemBlueprintLibrary.GetAbilitySystemComponent` (`.Target` (break `GameplayEventData` _payload)))))))))
          (:`OnCompleted`
            (`self.K2_EndAbility` :!label _label))
          (:`OnBlendOut`
            (goto _label))
          (:`OnInterrupted`
            (goto _label))
          (:`OnCancelled`
            (goto _label)))))
    (else
      (`self.K2_EndAbility`))))

(event `self.K2_OnEndAbility`
  (params (bWasCancelled :type Boolean)))